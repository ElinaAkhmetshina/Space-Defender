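; BP_DefenceZone is a defence zone that gives enemies standing positions on an arc around it and passes damage to the player.
; BuildSlots spreads slot locations evenly across the arc around the forward vector, showing them as instanced markers in construction and at BeginPlay.
; ClaimSlot assigns an enemy the nearest slot without a valid owner, returning its location or a not-found result.
; DamageZone forwards a damage amount to BP_Player's TakeHit.
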(event Custom|DamageZone
  (params (Amount :type Integer))
  (bind _asbp_player (Utilities|Casting|CastToBP_Player (Game|Player|GetPlayerPawn 0)))
  (Default|TakeHit _asbp_player Amount))

(event EventBeginPlay
  (CallFunction|BuildSlots)
  (Utilities|Array|Resize (Variables|State|GetSlotOwners) (Variables|Tuning|GetSlotCount)))

(event Collision|EventActorBeginOverlap
  (params (OtherActor :type Actor%20Object%20Reference)))

(event EventTick
  (params (DeltaSeconds :type Float%20%28single-precision%29)))

(fn ConstructionScript
  (CallFunction|BuildSlots))

(fn ClaimSlot
  (params (Enemy :type Actor%20Object%20Reference))
  (Variables|Default|SetBestIndex -1)
  (Variables|Default|SetBestDistance 999999.0)
  (for (_array_element _array_index) (Variables|State|GetSlotLocations)
    (if (and (< (Math|Vector|Distance(Vector) _array_element (Transformation|GetActorLocation Enemy)) (Variables|Default|GetBestDistance)) (not (Utilities|IsValid (Utilities|Array|Get(acopy) (Variables|State|GetSlotOwners) _array_index))))
      (Variables|Default|SetBestIndex _array_index)
      (Variables|Default|SetBestDistance (Math|Vector|Distance(Vector) _array_element (Transformation|GetActorLocation Enemy)))))
  (if (>= (Variables|Default|GetBestIndex) 0)
    (Utilities|Array|SetArrayElem (Variables|State|GetSlotOwners) (Variables|Default|GetBestIndex) Enemy true)
    (return true (Utilities|Array|Get(acopy) (Variables|State|GetSlotLocations) (Variables|Default|GetBestIndex)))
    (else
      (return false "0, 0, 0"))))

(fn BuildSlots
  (bind _slotcount (Variables|Tuning|GetSlotCount))
  (bind _returnvalue (- _slotcount 1))
  (Components|InstancedStaticMesh|ClearInstances (Variables|Default|GetSlotMarkers))
  (Utilities|Array|Clear (Variables|State|GetSlotLocations))
  (for _index (range 0 (Math|Float|Truncate _returnvalue))
    (Utilities|Array|Add (Variables|State|GetSlotLocations) (+ (Transformation|GetActorLocation) (* (Math|Vector|RotateVectorAroundAxis (Transformation|GetActorForwardVector) (+ (* _index (/ (Variables|Tuning|GetArcAngle) _returnvalue)) (* (Variables|Tuning|GetArcAngle) -0.5)) "0.000000,0.000000,1.000000") (Variables|Tuning|GetRadius))))
    (Components|InstancedStaticMesh|AddInstance (Variables|Default|GetSlotMarkers) (Math|Transform|MakeTransform (+ (Transformation|GetActorLocation) (* (Math|Vector|RotateVectorAroundAxis (Transformation|GetActorForwardVector) (+ (* _index (/ (Variables|Tuning|GetArcAngle) _returnvalue)) (* (Variables|Tuning|GetArcAngle) -0.5)) "0.000000,0.000000,1.000000") (Variables|Tuning|GetRadius))) "0, 0, 0" "0.300000,0.300000,0.300000") true)))