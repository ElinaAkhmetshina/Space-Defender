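; Player Blueprint with a crosshair-aimed gun, ammo, health and defeat handling.
; BeginPlay copies tuning from Stats and creates the HUD, whose crosshair position drives a Visibility trace for the aim point.
; Tick eases the gun pivot toward that point, while TryShoot spawns bullets aimed from the muzzle, with delay-based cooldown and automatic reload when empty.
; TakeHit updates health and at zero pauses the game and shows the defeat screen.
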(event Custom|TryShoot
  (bind _muzzle (Variables|Components|GetMuzzle))
  (bind _returnvalue (Transformation|GetWorldLocation _muzzle))
  (if (and (and (Variables|State|GetCanShoot) (> (Variables|State|GetAmmo) 0)) (not (Variables|State|GetIsReloading)))
    (Variables|State|SetAmmo (- (Variables|State|GetAmmo) 1))
    (Game|SpawnActorfromClass "/Game/BluePrints/BP_Bullet.BP_Bullet_C" (Math|Transform|MakeTransform _returnvalue (Math|Rotator|FindLookatRotation _returnvalue (CallFunction|GetAimPoint))) "AlwaysSpawn" "MultiplyWithRoot" 0 (Variables|Tuning|GetShotDamage) 0)
    (Default|UpdateAmmo (Variables|Default|GetHUD_Ref) (Variables|State|GetAmmo) (Variables|Tuning|GetMaxAmmo))
    (Variables|State|SetCanShoot false)
    (Utilities|FlowControl|Delay (Variables|Tuning|GetFireCooldown))
    (Variables|State|SetCanShoot true)
    (if (<= (Variables|State|GetAmmo) 0)
      (CallFunction|Reload))))

(event Custom|Reload
  (if (and (not (Variables|State|GetIsReloading)) (< (Variables|State|GetAmmo) (Variables|Tuning|GetMaxAmmo)))
    (Variables|State|SetIsReloading true)
    (Default|StartReloadUI (Variables|Default|GetHUD_Ref))
    (Utilities|FlowControl|Delay (Variables|Tuning|GetReloadTime))
    (Variables|State|SetAmmo (Variables|Tuning|GetMaxAmmo))
    (Variables|State|SetIsReloading false)
    (Default|UpdateAmmo (Variables|Default|GetHUD_Ref) (Variables|State|GetAmmo) (Variables|Tuning|GetMaxAmmo))))

(event Custom|GameOver
  (Game|SetGamePaused true)
  (Widget|SetVisibility (Variables|Default|GetHUD_Ref) "Collapsed")
  (bind _returnvalue (UserInterface|CreateWidget "/Game/UI/WBP_Defeat.WBP_Defeat_C" (Game|GetPlayerController 0)))
  (UserInterface|Viewport|AddtoViewport _returnvalue 0))

(event Custom|TakeHit
  (params (Damage :type Integer))
  (if (> (Variables|State|GetHealth) 0)
    (bind _output_get (Variables|State|SetHealth (Math|Integer|Max(Integer) (- (Variables|State|GetHealth) Damage))))
    (Default|UpdateHealth (Variables|Default|GetHUD_Ref) _output_get)
    (if (<= (Variables|State|GetHealth) 0)
      (CallFunction|GameOver))))

(event EventBeginPlay
  (bind _returnvalue (Game|GetPlayerController 0))
  (bind _stats (Variables|Data|GetStats))
  (if (Utilities|IsValid (Variables|Data|GetStats))
    (Variables|Tuning|SetMaxHealth (Variables|/Game/Data/PDA_PlayerStats.PDA_PlayerStats_C|GetMaxHealth _stats))
    (Variables|Tuning|SetMaxAmmo (Variables|/Game/Data/PDA_PlayerStats.PDA_PlayerStats_C|GetMaxAmmo _stats))
    (Variables|Tuning|SetReloadTime (Variables|/Game/Data/PDA_PlayerStats.PDA_PlayerStats_C|GetReloadTime _stats))
    (Variables|Tuning|SetFireCooldown (Variables|/Game/Data/PDA_PlayerStats.PDA_PlayerStats_C|GetFireCooldown _stats))
    (Variables|Tuning|SetShotDamage (Variables|/Game/Data/PDA_PlayerStats.PDA_PlayerStats_C|GetShotDamage _stats))
    (Variables|Tuning|SetShotRange (Variables|/Game/Data/PDA_PlayerStats.PDA_PlayerStats_C|GetShotRange _stats))
    (Variables|Tuning|SetGunTurnSpeed (Variables|/Game/Data/PDA_PlayerStats.PDA_PlayerStats_C|GetGunTurnSpeed _stats))
    (Variables|State|SetHealth (Variables|Tuning|GetMaxHealth))
    (Variables|State|SetAmmo (Variables|Tuning|GetMaxAmmo))
    (bind _returnvalue_2 (UserInterface|CreateWidget "/Game/UI/WBP_HUD.WBP_HUD_C" _returnvalue))
    (bind _output_get (Variables|Default|SetHUD_Ref _returnvalue_2))
    (UserInterface|Viewport|AddtoViewport _output_get 0)
    (Input|SetInputModeGameOnly _returnvalue false)
    (Default|UpdateAmmo (Variables|Default|GetHUD_Ref) (Variables|State|GetAmmo) (Variables|Tuning|GetMaxAmmo))
    (else
      (Development|PrintString "Missing player stats"))))

(event Collision|EventActorBeginOverlap
  (params (OtherActor :type Actor%20Object%20Reference)))

(event EventTick
  (params (DeltaSeconds :type Float%20%28single-precision%29))
  (Transformation|SetWorldRotation (Variables|Components|GetGunPivot) (Math|Interpolation|RInterpTo (Transformation|GetWorldRotation (Variables|Components|GetGunPivot)) (Math|Rotator|FindLookatRotation (Transformation|GetWorldLocation (Variables|Components|GetGunPivot)) (CallFunction|GetAimPoint)) (Utilities|Time|GetWorldDeltaSeconds) (Variables|Tuning|GetGunTurnSpeed)) false false))

(fn ConstructionScript)

(fn GetAimPoint
  (bind _returnvalue (Game|GetPlayerController 0))
  (bind _hud_ref (Variables|Default|GetHUD_Ref))
  (bind _shotrange (Variables|Tuning|GetShotRange))
  (bind _screenpos (Default|GetCrosshairScreenPos _hud_ref))
  (bind (_worldposition _worlddirection) (Class|GameplayStatics|DeprojectScreentoWorld _returnvalue _screenpos))
  (bind _returnvalue_2 (* _worlddirection _shotrange))
  (bind _returnvalue_3 (+ _returnvalue_2 _worldposition))
  (bind _outhit (Collision|LineTraceByChannel _worldposition _returnvalue_3 "TraceTypeQuery1" false 0 "ForOneFrame"))
  (return (select (.bBlockingHit (Collision|BreakHitResult _outhit)) (.ImpactPoint (Collision|BreakHitResult _outhit)) _returnvalue_3)))