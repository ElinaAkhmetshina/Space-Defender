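; BP_EnemyProjectile is an enemy projectile that damages the defence zone when it gets close to the player's camera.
; On BeginPlay it sets its lifespan and launches along its forward vector through the ProjectileMovement component.
; Each Tick compares its distance to the camera against HitDistance instead of using overlap events.
; On a hit it calls DamageZone on the BP_DefenceZone found by GetActorOfClass, then destroys itself.
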(event EventBeginPlay
  (Actor|SetLifeSpan (Variables|Tuning|GetLifeTime))
  (Variables|/Script/Engine.MovementComponent|SetVelocity (Variables|Default|GetProjectileMovement) (* (Transformation|GetActorForwardVector) (Variables|Default|GetSpeed))))

(event Collision|EventActorBeginOverlap
  (params (OtherActor :type Actor%20Object%20Reference)))

(event EventTick
  (params (DeltaSeconds :type Float%20%28single-precision%29))
  (if (<= (Math|Vector|Distance(Vector) (Transformation|GetActorLocation) (Camera|GetCameraLocation (Game|GetPlayerCameraManager 0))) (Variables|Tuning|GetHitDistance))
    (bind _returnvalue (Actor|GetActorOfClass "/Game/BluePrints/BP_DefenceZone.BP_DefenceZone_C"))
    (Default|DamageZone _returnvalue (Variables|Tuning|GetDamage))
    (Actor|DestroyActor)))

(fn ConstructionScript)