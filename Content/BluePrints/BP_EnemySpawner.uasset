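; BP_EnemySpawner periodically spawns random enemy types inside a box area, facing the defence zone.
; StartSpawning copies enemy types, interval, alive cap and count class from a config, then starts a looping timer after a start delay.
; Each tick of that timer spawns only while the count of CountClass actors is below the cap, yawing the enemy toward BP_DefenceZone.
; StopSpawning clears the timer.
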(event Custom|TrySpawn
  (bind _spawnarea (Variables|Default|GetSpawnArea))
  (bind _outactors (Actor|GetAllActorsOfClass (Variables|Tuning|GetCountClass)))
  (if (< (Utilities|Array|Length _outactors) (Variables|Tuning|GetMaxAlive))
    (bind _output_get (Variables|Default|SetSpawnPoint (Math|Random|RandomPointinBoundingBox (Transformation|GetWorldLocation _spawnarea) (Components|Box|GetScaledBoxExtent _spawnarea))))
    (bind _returnvalue (Actor|GetActorOfClass "/Game/BluePrints/BP_DefenceZone.BP_DefenceZone_C"))
    (Game|SpawnActorfromClass (.OutItem (Utilities|Array|Random (Variables|Tuning|GetEnemyTypes))) (Math|Transform|MakeTransform _output_get (Math|Rotator|MakeRotator 0.0 0.0 (.yaw (Math|Rotator|FindLookatRotation (Variables|Default|GetSpawnPoint) (Transformation|GetActorLocation _returnvalue))))) "AdjustIfPossibleButAlwaysSpawn" "MultiplyWithRoot" 0 0)))

(event Custom|StartSpawning
  (params (Config :type S%20Spawner%20Config%20Structure))
  (Variables|Tuning|SetEnemyTypes (.enemytypes Config))
  (bind _output_get (Variables|Tuning|SetSpawnInterval (.spawninterval Config)))
  (Variables|Tuning|SetMaxAlive (.maxalive Config))
  (Variables|Tuning|SetCountClass (.countclass Config))
  (Utilities|FlowControl|Delay (.startdelay Config))
  (bind _returnvalue (Utilities|Time|SetTimerbyEvent (delegate Custom|TrySpawn) _output_get true))
  (Variables|Default|SetSpawnTimer _returnvalue))

(event Custom|StopSpawning
  (Utilities|Time|ClearandInvalidateTimerbyHandle (Variables|Default|GetSpawnTimer)))

(event Collision|EventActorBeginOverlap
  (params (OtherActor :type Actor%20Object%20Reference)))

(event EventTick
  (params (DeltaSeconds :type Float%20%28single-precision%29)))

(fn ConstructionScript)