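; Flying demon enemy that hops between fly points and fires projectiles at the player's camera.
; A latent state machine in EnterState cycles fly, wind-up, shoot and cooldown, relocating after a set number of shots; Tick handles movement.
; It reserves a random free BP_FlyPoint through its Occupant, releasing it on death.
; Tuning comes from a stats data asset; shots require range, view-cone, line-of-sight and recently-rendered checks.
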(event Custom|EnterState
  (params (NewState :type E_FlyerState%20Enum :default "NewEnumerator0"))
  (bind _output_get (Variables|State|SetState NewState))
  (switch Utilities|FlowControl|Switch|SwitchonE_FlyerState _output_get
    (:NewEnumerator0
      (bind (_found _point) (CallFunction|PickFlyPoint))
      (if _found
        (if (Utilities|IsValid (Variables|State|GetCurrentPoint))
          (Variables|/Game/BluePrints/BP_FlyPoint.BP_FlyPoint_C|SetOccupant (Variables|State|GetCurrentPoint) 0))
        (Variables|/Game/BluePrints/BP_FlyPoint.BP_FlyPoint_C|SetOccupant _point self)
        (Variables|State|SetCurrentPoint _point)
        (Variables|State|SetShotsFired 0)
        (CallFunction|PlayLoop "/Game/Assets/Monsters/Demon/DemonCharacterArmature_Fast_Flying.DemonCharacterArmature_Fast_Flying")
        (else
          (CallFunction|PlayLoop "/Game/Assets/Monsters/Demon/DemonCharacterArmature_Flying_Idle.DemonCharacterArmature_Flying_Idle")
          (Utilities|FlowControl|Delay 1.0)
          (if (Utilities|Enum|Equal(Enum) (Variables|State|GetState) "NewEnumerator0")
            (CallFunction|EnterState "NewEnumerator0")))))
    (:NewEnumerator1
      (Transformation|SetActorRotation (Math|Rotator|MakeRotator 0.0 0.0 (.yaw (Math|Rotator|FindLookatRotation (Transformation|GetActorLocation) (Camera|GetCameraLocation (Game|GetPlayerCameraManager 0))))))
      (CallFunction|PlayLoop "/Game/Assets/Monsters/Demon/DemonCharacterArmature_Yes.DemonCharacterArmature_Yes")
      (Utilities|FlowControl|Delay (Variables|Tuning|GetWindUpTime))
      (if (Utilities|Enum|Equal(Enum) (Variables|State|GetState) "NewEnumerator1")
        (CallFunction|EnterState "NewEnumerator2")))
    (:NewEnumerator2
      (bind _cansee (CallFunction|CanSeePlayer))
      (if (and _cansee (Class|Actor|WasRecentlyRendered 0.2))
        (Components|Animation|PlayAnimation (Variables|Character|GetMesh) "/Game/Assets/Monsters/Demon/DemonCharacterArmature_Punch.DemonCharacterArmature_Punch" false)
        (Utilities|FlowControl|Delay (Variables|Tuning|GetProjectileReleaseTime))
        (if (Utilities|Enum|Equal(Enum) (Variables|State|GetState) "NewEnumerator2")
          (bind _output_get_2 (Variables|Default|SetSpawnPos (+ (Transformation|GetActorLocation) (* (Transformation|GetActorForwardVector) 8e+01))))
          (Game|SpawnActorfromClass "/Game/BluePrints/BP_EnemyProjectile.BP_EnemyProjectile_C" (Math|Transform|MakeTransform _output_get_2 (Math|Rotator|FindLookatRotation (Variables|Default|GetSpawnPos) (Camera|GetCameraLocation (Game|GetPlayerCameraManager 0)))) "AlwaysSpawn" "MultiplyWithRoot" 0 (Variables|Tuning|GetAttackDamage) (Variables|Runtime|GetProjectileSpeed) 0)
          (Variables|State|SetShotsFired (+ (Variables|State|GetShotsFired) 1))
          (Utilities|FlowControl|Delay (- (Animation|GetPlayLength (Variables|Tuning|GetAnim_Punch)) (Variables|Tuning|GetProjectileReleaseTime)))
          (if (Utilities|Enum|Equal(Enum) (Variables|State|GetState) "NewEnumerator2")
            (CallFunction|EnterState "NewEnumerator3")))
        (else
          (CallFunction|EnterState "NewEnumerator0"))))
    (:NewEnumerator3
      (CallFunction|PlayLoop "/Game/Assets/Monsters/Demon/DemonCharacterArmature_Flying_Idle.DemonCharacterArmature_Flying_Idle")
      (Utilities|FlowControl|Delay (Variables|Tuning|GetAttackCooldown))
      (if (Utilities|Enum|Equal(Enum) (Variables|State|GetState) "NewEnumerator3")
        (if (>= (Variables|State|GetShotsFired) (Variables|Tuning|GetShotsBeforeMove))
          (CallFunction|EnterState "NewEnumerator0")
          (else
            (CallFunction|EnterState "NewEnumerator1")))))))

(event EventBeginPlay
  (bind _stats (Variables|Default|GetStats))
  (|CallParentFunction)
  (Variables|Tuning|SetAttackDamage (Variables|/Game/Data/PDA_EnemyStats.PDA_EnemyStats_C|GetAttackDamage _stats))
  (Variables|Tuning|SetAttackCooldown (Variables|/Game/Data/PDA_EnemyStats.PDA_EnemyStats_C|GetAttackCooldown _stats))
  (Variables|Tuning|SetWindUpTime (Variables|/Game/Data/PDA_EnemyStats.PDA_EnemyStats_C|GetWindUpTime _stats))
  (bind _aspda_flyer_stats (Utilities|Casting|CastToPDA_FlyerStats (Variables|Default|GetStats)))
  (Variables|Tuning|SetVisionRange (Variables|/Game/Data/PDA_FlyerStats.PDA_FlyerStats_C|GetVisionRange _aspda_flyer_stats))
  (Variables|Tuning|SetVisionAngle (Variables|/Game/Data/PDA_FlyerStats.PDA_FlyerStats_C|GetVisionAngle _aspda_flyer_stats))
  (Variables|Tuning|SetShotsBeforeMove (Variables|/Game/Data/PDA_FlyerStats.PDA_FlyerStats_C|GetShotsBeforeMove _aspda_flyer_stats))
  (Variables|Tuning|SetProjectileReleaseTime (Variables|/Game/Data/PDA_FlyerStats.PDA_FlyerStats_C|GetProjectileReleaseTime _aspda_flyer_stats))
  (Variables|Runtime|SetProjectileSpeed (Variables|/Game/Data/PDA_FlyerStats.PDA_FlyerStats_C|GetProjectileSpeed _aspda_flyer_stats))
  (Pawn|Components|CharacterMovement|SetMovementMode (Variables|Character|GetCharacterMovement) "MOVE_Flying" 0)
  (bind _returnvalue (Actor|GetActorOfClass "/Game/BluePrints/BP_DefenceZone.BP_DefenceZone_C"))
  (Variables|State|SetZone _returnvalue)
  (CallFunction|EnterState "NewEnumerator0"))

(event Collision|EventActorBeginOverlap
  (params (OtherActor :type Actor%20Object%20Reference))
  (|CallParentFunction OtherActor) ; This node is disabled and will not be called.\nDrag off pins to build functionality.
)

(event EventTick
  (params (DeltaSeconds :type Float%20%28single-precision%29))
  (|CallParentFunction DeltaSeconds)
  (if (and (Utilities|Enum|Equal(Enum) (Variables|State|GetState) "NewEnumerator0") (Utilities|IsValid (Variables|State|GetCurrentPoint)))
    (Transformation|SetActorLocation (Math|Interpolation|VInterptoConstant (Transformation|GetActorLocation) (Transformation|GetActorLocation (Variables|State|GetCurrentPoint)) (Utilities|Time|GetWorldDeltaSeconds) (Variables|Default|GetMoveSpeed)) false false)
    (Transformation|SetActorRotation (Math|Rotator|MakeRotator 0.0 0.0 (.yaw (Math|Rotator|FindLookatRotation (Transformation|GetActorLocation) (Transformation|GetActorLocation (Variables|State|GetCurrentPoint))))))
    (if (<= (Math|Vector|Distance(Vector) (Transformation|GetActorLocation) (Transformation|GetActorLocation (Variables|State|GetCurrentPoint))) (Variables|Tuning|GetAcceptanceRadius))
      (CallFunction|EnterState "NewEnumerator1"))))

(event EventDie
  (CallFunction|EnterState "NewEnumerator4")
  (if (Utilities|IsValid (Variables|State|GetCurrentPoint))
    (Variables|/Game/BluePrints/BP_FlyPoint.BP_FlyPoint_C|SetOccupant (Variables|State|GetCurrentPoint) 0))
  (|CallParentFunction))

(fn ConstructionScript
  (|CallParentFunction))

(fn CanSeePlayer
  (bind _returnvalue (Transformation|GetActorLocation))
  (bind _returnvalue_2 (Game|GetPlayerCameraManager 0))
  (bind _returnvalue_3 (Camera|GetCameraLocation _returnvalue_2))
  (bind _returnvalue_4 (+ _returnvalue "0.000000,0.000000,50.000000"))
  (bind _returnvalue_5 (- _returnvalue_3 _returnvalue_4))
  (bind _returnvalue_6 (Collision|LineTraceByChannel _returnvalue_4 _returnvalue_3 "TraceTypeQuery1" false 0 "None"))
  (return (and (and (>= (Math|Vector|DotProduct (Transformation|GetActorForwardVector) (Math|Vector|Normalize _returnvalue_5)) (Math|Trig|Cos(Degrees) (* (Variables|Tuning|GetVisionAngle) 0.5))) (<= (Math|Vector|VectorLength _returnvalue_5) (Variables|Tuning|GetVisionRange))) (not _returnvalue_6))))

(fn PickFlyPoint
  (Utilities|Array|Clear (LocalVariables|GetFreePoints))
  (bind _outactors (Actor|GetAllActorsOfClass "/Game/BluePrints/BP_FlyPoint.BP_FlyPoint_C"))
  (for _array_element _outactors
    (if (not (Utilities|IsValid (Variables|/Game/BluePrints/BP_FlyPoint.BP_FlyPoint_C|GetOccupant _array_element)))
      (bind _output_get (LocalVariables|SetFreePoints (LocalVariables|GetFreePoints)))
      (Utilities|Array|Add _output_get _array_element)))
  (if (> (Utilities|Array|Length (LocalVariables|GetFreePoints)) 0)
    (return true (.OutItem (Utilities|Array|Random (LocalVariables|GetFreePoints))))
    (else
      (return false 0))))