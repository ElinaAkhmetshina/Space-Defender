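; Enemy AI that dashes between hiding spots toward the defence zone, then claims a slot and attacks it.
; An enum state machine runs dash, hide, approach, cooldown, wind-up and attack with AIMoveTo and delays, tuned from a Speedster stats asset.
; A vision-cone and trace check on the player camera triggers sprinting or breaks hiding.
; Attacks resume the wind-up animation at normal speed, damaging the zone only if recently rendered.
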(event Custom|EnterState
  (params (NewState :type E_SpeedsterState%20Enum :default "NewEnumerator0"))
  (bind _output_get (Variables|State|SetState NewState))
  (switch Utilities|FlowControl|Switch|SwitchonE_SpeedsterState _output_get
    (:NewEnumerator0
      (bind (_found _cover) (CallFunction|FindNextCover))
      (if _found
        (bind _output_get_2 (Variables|State|SetCurrentCover _cover))
        (Utilities|Array|Add (Variables|State|GetVisitedCovers) _output_get_2)
        (CallFunction|PlayLoop "/Game/Assets/Monsters/Ghost/GhostCharacterArmature_Fast_Flying.GhostCharacterArmature_Fast_Flying")
        (AI|AIMoveTo self (Transformation|GetActorLocation (Variables|State|GetCurrentCover)) 0 (Variables|Tuning|GetAcceptanceRadius) false
          (:OnSuccess
            (if (Utilities|Enum|Equal(Enum) (Variables|State|GetState) "NewEnumerator0")
              (CallFunction|EnterState "NewEnumerator1")))
          (:OnFail
            (Utilities|FlowControl|Delay 0.2)
            (if (Utilities|Enum|Equal(Enum) (Variables|State|GetState) "NewEnumerator0")
              (CallFunction|EnterState "NewEnumerator0"))))
        (else
          (CallFunction|EnterState "NewEnumerator2"))))
    (:NewEnumerator1
      (CallFunction|PlayLoop "/Game/Assets/Monsters/Ghost/GhostCharacterArmature_Flying_Idle.GhostCharacterArmature_Flying_Idle")
      (Utilities|FlowControl|RetriggerableDelay (Variables|Tuning|GetHideTime))
      (if (Utilities|Enum|Equal(Enum) (Variables|State|GetState) "NewEnumerator1")
        (CallFunction|EnterState "NewEnumerator0")))
    (:NewEnumerator2
      (bind (_found_2 _location) (Default|ClaimSlot (Variables|State|GetZone) self))
      (if _found_2
        (Variables|State|SetSlotLocation _location)
        (Variables|/Script/Engine.CharacterMovementComponent|SetMaxWalkSpeed (Variables|Character|GetCharacterMovement) (Variables|Tuning|GetSprintSpeed))
        (CallFunction|PlayLoop "/Game/Assets/Monsters/Ghost/GhostCharacterArmature_Fast_Flying.GhostCharacterArmature_Fast_Flying")
        (AI|AIMoveTo self (Variables|State|GetSlotLocation) 0 (Variables|Tuning|GetAcceptanceRadius) false :!label _label
          (:OnSuccess
            (if (Utilities|Enum|Equal(Enum) (Variables|State|GetState) "NewEnumerator2")
              (Transformation|SetActorRotation (Math|Rotator|MakeRotator 0.0 0.0 (.yaw (Math|Rotator|FindLookatRotation (Transformation|GetActorLocation) (Transformation|GetActorLocation (Variables|State|GetZone))))))
              (CallFunction|EnterState "NewEnumerator3")))
          (:OnFail
            (Utilities|FlowControl|Delay 0.5)
            (if (Utilities|Enum|Equal(Enum) (Variables|State|GetState) "NewEnumerator2")
              (goto _label)
              (else
                (CallFunction|PlayLoop "/Game/Assets/Monsters/Ghost/GhostCharacterArmature_Flying_Idle.GhostCharacterArmature_Flying_Idle")
                (Utilities|FlowControl|Delay 1.0)
                (if (Utilities|Enum|Equal(Enum) (Variables|State|GetState) "NewEnumerator2")
                  (CallFunction|EnterState "NewEnumerator2"))))))))
    (:NewEnumerator3
      (CallFunction|PlayLoop "/Game/Assets/Monsters/Ghost/GhostCharacterArmature_Flying_Idle.GhostCharacterArmature_Flying_Idle")
      (Utilities|FlowControl|Delay (Variables|Tuning|GetAttackCooldown))
      (if (Utilities|Enum|Equal(Enum) (Variables|State|GetState) "NewEnumerator3")
        (CallFunction|EnterState "NewEnumerator4")))
    (:NewEnumerator4
      (bind _output_get_3 (Variables|State|SetCurrentAttackAnim (select (Math|Random|RandomBool) (Variables|Animation|GetAnim_Headbutt) (Variables|Animation|GetAnim_Punch))))
      (Components|Animation|PlayAnimation (Variables|Character|GetMesh) _output_get_3 false)
      (Components|Timeline|SetPlayRate (Variables|Character|GetMesh) (Variables|Tuning|GetWindUpPlayRate))
      (Utilities|FlowControl|Delay (Variables|Tuning|GetWindUpTime))
      (if (Utilities|Enum|Equal(Enum) (Variables|State|GetState) "NewEnumerator4")
        (CallFunction|EnterState "NewEnumerator5")))
    (:NewEnumerator5
      (Components|Animation|PlayAnimation (Variables|Character|GetMesh) (Variables|State|GetCurrentAttackAnim) false)
      (bind _output_get_4 (Variables|Default|SetWindUpPos (* (Variables|Tuning|GetWindUpTime) (Variables|Tuning|GetWindUpPlayRate))))
      (Components|Animation|SetPosition (Variables|Character|GetMesh) _output_get_4 false)
      (Components|Timeline|SetPlayRate (Variables|Character|GetMesh) 1.0)
      (Utilities|FlowControl|Delay (- (Animation|GetPlayLength (Variables|State|GetCurrentAttackAnim)) (Variables|Default|GetWindUpPos)))
      (if (Utilities|Enum|Equal(Enum) (Variables|State|GetState) "NewEnumerator5")
        (if (Class|Actor|WasRecentlyRendered 0.2)
          (Default|DamageZone (Variables|State|GetZone) (Variables|Tuning|GetAttackDamage))
          (CallFunction|EnterState "NewEnumerator3")
          (else
            (CallFunction|EnterState "NewEnumerator3")))))))

(event EventBeginPlay
  (bind _stats (Variables|Default|GetStats))
  (Variables|Tuning|SetAttackDamage (Variables|/Game/Data/PDA_EnemyStats.PDA_EnemyStats_C|GetAttackDamage _stats))
  (Variables|Tuning|SetAttackCooldown (Variables|/Game/Data/PDA_EnemyStats.PDA_EnemyStats_C|GetAttackCooldown _stats))
  (Variables|Tuning|SetWindUpTime (Variables|/Game/Data/PDA_EnemyStats.PDA_EnemyStats_C|GetWindUpTime _stats))
  (bind _aspda_speedster_stats (Utilities|Casting|CastToPDA_SpeedsterStats (Variables|Default|GetStats)))
  (Variables|/Game/Data/PDA_SpeedsterStats.PDA_SpeedsterStats_C|SetVisionRange _aspda_speedster_stats 0.0)
  (Variables|Tuning|SetVisionAngle (Variables|/Game/Data/PDA_SpeedsterStats.PDA_SpeedsterStats_C|GetVisionAngle _aspda_speedster_stats))
  (Variables|Tuning|SetHideTime (Variables|/Game/Data/PDA_SpeedsterStats.PDA_SpeedsterStats_C|GetHideTime _aspda_speedster_stats))
  (Variables|Tuning|SetSprintSpeed (Variables|/Game/Data/PDA_SpeedsterStats.PDA_SpeedsterStats_C|GetSprintSpeed _aspda_speedster_stats))
  (Variables|Tuning|SetWindUpPlayRate (Variables|/Game/Data/PDA_SpeedsterStats.PDA_SpeedsterStats_C|GetWindUpPlayRate _aspda_speedster_stats))
  (|CallParentFunction)
  (bind _returnvalue (Actor|GetActorOfClass "/Game/BluePrints/BP_DefenceZone.BP_DefenceZone_C"))
  (Variables|State|SetZone _returnvalue)
  (CallFunction|EnterState "NewEnumerator0")
  (CallFunction|FindNextCover))

(event Collision|EventActorBeginOverlap
  (params (OtherActor :type Actor%20Object%20Reference))
  (|CallParentFunction OtherActor) ; This node is disabled and will not be called.\nDrag off pins to build functionality.
)

(event EventTick
  (params (DeltaSeconds :type Float%20%28single-precision%29))
  (|CallParentFunction DeltaSeconds)
  (if (Utilities|Enum|Equal(Enum) (Variables|State|GetState) "NewEnumerator0")
    (bind _cansee (CallFunction|CanSeePlayer))
    (Variables|State|SetIsExposed _cansee)
    (Variables|/Script/Engine.CharacterMovementComponent|SetMaxWalkSpeed (Variables|Character|GetCharacterMovement) (Math|Float|SelectFloat (Variables|Tuning|GetSprintSpeed) (Variables|Default|GetMoveSpeed) _cansee))
    (elif (Utilities|Enum|Equal(Enum) (Variables|State|GetState) "NewEnumerator1")
      (bind _cansee_2 (CallFunction|CanSeePlayer))
      (if _cansee_2
        (CallFunction|EnterState "NewEnumerator0")))))

(event EventDie
  (CallFunction|EnterState "NewEnumerator6")
  (|CallParentFunction))

(fn ConstructionScript
  (|CallParentFunction))

(fn CanSeePlayer
  (bind _returnvalue (Transformation|GetActorLocation))
  (bind _returnvalue_2 (Game|GetPlayerCameraManager 0))
  (bind _returnvalue_3 (Camera|GetCameraLocation _returnvalue_2))
  (bind _returnvalue_4 (+ _returnvalue "0.000000,0.000000,50.000000"))
  (bind _returnvalue_5 (- _returnvalue_3 _returnvalue_4))
  (bind _returnvalue_6 (Collision|LineTraceByChannel _returnvalue_4 _returnvalue_3 "TraceTypeQuery1" false 0 "None"))
  (return (and (and (>= (Math|Vector|DotProduct (Transformation|GetActorForwardVector) (Math|Vector|Normalize _returnvalue_5)) (Math|Trig|Cos(Degrees) (* (Variables|Tuning|GetVisionAngle) 0.5))) (<= (Math|Vector|VectorLength _returnvalue_5) (Variables|Tuning|GetVisionRange))) (not _returnvalue_6))))

(fn FindNextCover
  (Variables|Default|SetBestCover 0)
  (Variables|Default|SetBestDistance 9999999.0)
  (bind _outactors (Actor|GetAllActorsOfClass "/Game/BluePrints/BP_HidingSpot.BP_HidingSpot_C"))
  (for _array_element _outactors
    (if (Math|Boolean|ANDBoolean (< (Math|Vector|Distance(Vector) (Transformation|GetActorLocation _array_element) (Transformation|GetActorLocation)) (Variables|Default|GetBestDistance)) (not (Utilities|Array|ContainsItem (Variables|State|GetVisitedCovers) _array_element)) (< (Math|Vector|Distance(Vector) (Transformation|GetActorLocation _array_element) (Transformation|GetActorLocation (Variables|State|GetZone))) (Math|Vector|Distance(Vector) (Transformation|GetActorLocation) (Transformation|GetActorLocation (Variables|State|GetZone)))))
      (Variables|Default|SetBestCover _array_element)
      (Variables|Default|SetBestDistance (Math|Vector|Distance(Vector) (Transformation|GetActorLocation _array_element) (Transformation|GetActorLocation)))))
  (return (Utilities|IsValid (Variables|Default|GetBestCover)) (Variables|Default|GetBestCover)))