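; BP_EnemyBase is a base enemy character that handles health, hit reactions and death.
; On BeginPlay it copies health, speed and scale from a Stats object, or prints a warning if that is missing.
; Animations play directly on the mesh without state logic: one-shots return to the current loop after a retriggerable delay.
; Damage plays a hit reaction, while death disables movement and capsule collision, then sets a lifespan from the death animation's length.
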(event Custom|PlayLoop
  (params (Anim :type Anim%20Sequence%20Object%20Reference))
  (bind _output_get (Variables|State|SetCurrentLoopAnim Anim))
  (Components|Animation|PlayAnimation (Variables|Character|GetMesh) _output_get true)
  (Components|Timeline|SetPlayRate (Variables|Character|GetMesh) 1.0))

(event Custom|PlayOnce
  (params (Anim :type Anim%20Sequence%20Object%20Reference))
  (Components|Animation|PlayAnimation (Variables|Character|GetMesh) Anim false)
  (Components|Timeline|SetPlayRate (Variables|Character|GetMesh) 1.0)
  (Utilities|FlowControl|RetriggerableDelay (Animation|GetPlayLength Anim))
  (if (not (Variables|State|GetIsDead))
    (Components|Animation|PlayAnimation (Variables|Character|GetMesh) (Variables|State|GetCurrentLoopAnim) true)
    (Components|Timeline|SetPlayRate (Variables|Character|GetMesh) 1.0)))

(event Custom|Die
  (bind _anim_death (Variables|Animation|GetAnim_Death))
  (Variables|State|SetIsDead true)
  (Pawn|Components|CharacterMovement|DisableMovement (Variables|Character|GetCharacterMovement))
  (Collision|SetCollisionEnabled (Variables|Collision|GetCapsuleComponent) "NoCollision")
  (Components|Animation|PlayAnimation (Variables|Character|GetMesh) _anim_death false)
  (Actor|SetLifeSpan (+ (Animation|GetPlayLength _anim_death) 1.0)))

(event EventBeginPlay
  (if (Utilities|IsValid (Variables|Data|GetStats))
    (Variables|Tuning|SetMaxHealth (Variables|/Game/Data/PDA_EnemyStats.PDA_EnemyStats_C|GetMaxHealth (Variables|Data|GetStats)))
    (Variables|Tuning|SetMoveSpeed (Variables|/Game/Data/PDA_EnemyStats.PDA_EnemyStats_C|GetMoveSpeed (Variables|Data|GetStats)))
    (Transformation|SetActorScale3D (Math|Conversions|ToVector(Float) (Variables|/Game/Data/PDA_EnemyStats.PDA_EnemyStats_C|GetScale (Variables|Data|GetStats))))
    (Variables|State|SetHealth (Variables|Tuning|GetMaxHealth))
    (Variables|/Script/Engine.CharacterMovementComponent|SetMaxWalkSpeed (Variables|Character|GetCharacterMovement) (Variables|Tuning|GetMoveSpeed))
    (CallFunction|PlayLoop (Variables|Animation|GetAnim_Idle))
    (else
      (Development|PrintString (Utilities|String|Append "Missing stats on " (Utilities|GetDisplayName self))))))

(event Collision|EventActorBeginOverlap
  (params (OtherActor :type Actor%20Object%20Reference)))

(event EventTick
  (params (DeltaSeconds :type Float%20%28single-precision%29)))

(event Game|Damage|EventAnyDamage
  (params (Damage :type Float%20%28single-precision%29) (DamageType :type Damage%20Type%20Object%20Reference) (InstigatedBy :type Controller%20Object%20Reference) (DamageCauser :type Actor%20Object%20Reference))
  (if (not (Variables|State|GetIsDead))
    (Variables|State|SetHealth (- (Variables|State|GetHealth) Damage))
    (if (<= (Variables|State|GetHealth) 0.0)
      (CallFunction|Die)
      (else
        (CallFunction|PlayOnce (Variables|Animation|GetAnim_Hit))))))

(fn ConstructionScript)