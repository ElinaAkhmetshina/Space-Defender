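; Level manager actor that runs the selected level: enemy spawning, timed goal, score and level completion.
; On BeginPlay it reads level data from the game instance (or its default), starts tag-matched spawners, initializes the player's HUD and optionally shows a paused tutorial.
; Tick counts down timed goals to LevelComplete, which, given a next level, saves progress, stops spawners, pauses and shows victory.
; Separate events add score and save best score.
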(event Custom|LevelComplete
  (if (not (Variables|Default|GetIsLevelOver))
    (Variables|Default|SetIsLevelOver true)
    (if (Utilities|IsValid (Variables|/Game/Data/PDA_LevelData.PDA_LevelData_C|GetNextLevel (Variables|Default|GetLevelData)))
      (bind _asbp_game_instance (Utilities|Casting|CastToBP_GameInstance (Game|GetGameInstance)))
      (Variables|/Game/BluePrints/BP_SaveData.BP_SaveData_C|SetCurrentLevelIndex (Variables|/Game/BluePrints/BP_GameInstance.BP_GameInstance_C|GetSaveRef _asbp_game_instance) (Variables|/Game/Data/PDA_LevelData.PDA_LevelData_C|GetLevelIndex (Variables|/Game/Data/PDA_LevelData.PDA_LevelData_C|GetNextLevel (Variables|Default|GetLevelData))))
      (Default|SaveGame _asbp_game_instance)
      (bind _outactors (Actor|GetAllActorsOfClass "/Game/BluePrints/BP_EnemySpawner.BP_EnemySpawner_C"))
      (for _array_element _outactors
        (Default|StopSpawning _array_element))
      (Game|SetGamePaused true)
      (Widget|SetVisibility (CallFunction|GetHUD) "Collapsed")
      (bind _returnvalue (UserInterface|CreateWidget "/Game/UI/WBP_Victory.WBP_Victory_C" (Game|GetPlayerController 0) (Variables|/Game/Data/PDA_LevelData.PDA_LevelData_C|GetNextLevel (Variables|Default|GetLevelData))))
      (UserInterface|Viewport|AddtoViewport _returnvalue 0))))

(event Custom|AddScore
  (params (Amount :type Integer))
  (if (not (Variables|Default|GetIsLevelOver))
    (bind _output_get (Variables|Default|SetScore (+ (Variables|Default|GetScore) Amount)))
    (Default|UpdateScore (CallFunction|GetHUD) _output_get)))

(event Custom|SaveBestScore
  (bind _score (Variables|Default|GetScore))
  (bind _asbp_game_instance (Utilities|Casting|CastToBP_GameInstance (Game|GetGameInstance)))
  (if (> _score (Variables|/Game/BluePrints/BP_SaveData.BP_SaveData_C|GetBestScore (Variables|/Game/BluePrints/BP_GameInstance.BP_GameInstance_C|GetSaveRef _asbp_game_instance)))
    (Variables|/Game/BluePrints/BP_SaveData.BP_SaveData_C|SetBestScore (Variables|/Game/BluePrints/BP_GameInstance.BP_GameInstance_C|GetSaveRef _asbp_game_instance) _score)
    (Default|SaveGame _asbp_game_instance)))

(event EventBeginPlay
  (bind _hud (CallFunction|GetHUD))
  (bind _asbp_game_instance (Utilities|Casting|CastToBP_GameInstance (Game|GetGameInstance)))
  (Variables|Default|SetLevelData (select (Utilities|IsValid (Variables|/Game/BluePrints/BP_GameInstance.BP_GameInstance_C|GetSelectedLevel _asbp_game_instance)) (Variables|/Game/BluePrints/BP_GameInstance.BP_GameInstance_C|GetSelectedLevel _asbp_game_instance) (Variables|/Game/BluePrints/BP_GameInstance.BP_GameInstance_C|GetDefaultLevel _asbp_game_instance)))
  (for _array_element (Variables|/Game/Data/PDA_LevelData.PDA_LevelData_C|GetSpawners (Variables|Default|GetLevelData))
    (bind _outactors (Actor|GetAllActorsOfClasswithTag "/Game/BluePrints/BP_EnemySpawner.BP_EnemySpawner_C" (.SpawnerTag (Utilities|Struct|BreakS_SpawnerConfig _array_element))))
    (for _array_element_2 _outactors
      (Default|StartSpawning _array_element_2 _array_element))
    (Variables|Default|SetTimeLeft (Variables|/Game/Data/PDA_LevelData.PDA_LevelData_C|GetTimeLimit (Variables|Default|GetLevelData)))
    (Utilities|FlowControl|DelayUntilNextTick)
    (Default|SetGoalMode _hud (Utilities|Enum|Equal(Enum) (Variables|/Game/Data/PDA_LevelData.PDA_LevelData_C|GetGoal (Variables|Default|GetLevelData)) "NewEnumerator0"))
    (Default|UpdateTimer _hud (Variables|Default|GetTimeLeft))
    (Default|UpdateScore _hud)
    (if (Variables|/Game/Data/PDA_LevelData.PDA_LevelData_C|GetShowTutorial (Variables|Default|GetLevelData))
      (bind _returnvalue (UserInterface|CreateWidget "/Game/UI/WBP_Tutorial.WBP_Tutorial_C" (Game|GetPlayerController 0)))
      (UserInterface|Viewport|AddtoViewport _returnvalue 10)
      (Game|SetGamePaused true))))

(event Collision|EventActorBeginOverlap
  (params (OtherActor :type Actor%20Object%20Reference)))

(event EventTick
  (params (DeltaSeconds :type Float%20%28single-precision%29))
  (if (and (Utilities|Enum|Equal(Enum) (Variables|/Game/Data/PDA_LevelData.PDA_LevelData_C|GetGoal (Variables|Default|GetLevelData)) "NewEnumerator0") (not (Variables|Default|GetIsLevelOver)))
    (bind _output_get (Variables|Default|SetTimeLeft (Math|Float|Max(Float) (- (Variables|Default|GetTimeLeft) (Utilities|Time|GetWorldDeltaSeconds)) 0.0)))
    (Default|UpdateTimer (CallFunction|GetHUD) _output_get)
    (if (<= (Variables|Default|GetTimeLeft) 0.0)
      (CallFunction|LevelComplete))))

(fn ConstructionScript)

(fn GetHUD
  (return (Variables|/Game/BluePrints/BP_Player.BP_Player_C|GetHUD_Ref (.AsBP%20Player (Utilities|Casting|CastToBP_Player (Game|Player|GetPlayerPawn 0))))))