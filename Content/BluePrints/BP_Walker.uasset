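; BP_Walker is an enemy that walks to a slot at the defence zone and repeatedly bites to damage it.
; It loads combat stats, claims a slot from BP_DefenceZone, retrying until one is free, then moves there with AI MoveTo.
; An EnterState state machine cycles Cooldown, Wind Up and Attack using delays, animations and sounds, stopping on death.
; Bites only deal damage if the walker was recently rendered.
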(event Custom|TryClaimSlot
  (bind (_found _location) (Default|ClaimSlot (Variables|State|GetZone) self))
  (if _found
    (Variables|State|SetSlotLocation _location)
    (CallFunction|EnterState "NewEnumerator0")
    (else
      (CallFunction|PlayLoop "/Game/Assets/Monsters/Spiky/GreenSpikyBlobCharacterArmature_Idle.GreenSpikyBlobCharacterArmature_Idle")
      (Utilities|FlowControl|Delay 1.0)
      (CallFunction|TryClaimSlot))))

(event Custom|EnterState
  (params (NewState :type E_WalkerState%20Enum :default "NewEnumerator0"))
  (bind _output_get (Variables|State|SetState NewState))
  (switch Utilities|FlowControl|Switch|SwitchonE_WalkerState _output_get
    (:NewEnumerator0
      (CallFunction|PlayLoop)
      (AI|AIMoveTo self (Variables|State|GetSlotLocation) 0 (Variables|Tuning|GetAcceptanceRadius) false
        (:OnSuccess
          (if (not (Variables|Default|GetIsDead))
            (Transformation|SetActorRotation (Math|Rotator|MakeRotator 0.0 0.0 (.yaw (Math|Rotator|FindLookatRotation (Transformation|GetActorLocation) (Transformation|GetActorLocation (Variables|State|GetZone))))))
            (CallFunction|EnterState "NewEnumerator1")))
        (:OnFail
          (if (not (Variables|Default|GetIsDead))
            (Utilities|FlowControl|Delay 0.5)
            (CallFunction|EnterState "NewEnumerator0")))))
    (:NewEnumerator1
      (CallFunction|PlayLoop "/Game/Assets/Monsters/Spiky/GreenSpikyBlobCharacterArmature_Idle.GreenSpikyBlobCharacterArmature_Idle")
      (Utilities|FlowControl|Delay (Variables|Tuning|GetAttackCooldown))
      (if (not (Variables|Default|GetIsDead))
        (CallFunction|EnterState "NewEnumerator2")))
    (:NewEnumerator2
      (CallFunction|PlayEnemySound (Variables|/Game/Data/PDA_EnemyStats.PDA_EnemyStats_C|GetSound_WindUp (Variables|Default|GetStats)))
      (CallFunction|PlayLoop "/Game/Assets/Monsters/Spiky/GreenSpikyBlobCharacterArmature_Dance.GreenSpikyBlobCharacterArmature_Dance")
      (Utilities|FlowControl|Delay (Variables|Tuning|GetWindUpTime))
      (if (not (Variables|Default|GetIsDead))
        (CallFunction|EnterState "NewEnumerator3")))
    (:NewEnumerator3
      (CallFunction|PlayEnemySound (Variables|/Game/Data/PDA_EnemyStats.PDA_EnemyStats_C|GetSound_Attack (Variables|Default|GetStats)))
      (Components|Animation|PlayAnimation (Variables|Character|GetMesh) "/Game/Assets/Monsters/Spiky/GreenSpikyBlobCharacterArmature_Bite_Front.GreenSpikyBlobCharacterArmature_Bite_Front" false)
      (Utilities|FlowControl|Delay 0.2)
      (if (not (Variables|Default|GetIsDead))
        (if (Class|Actor|WasRecentlyRendered 0.2)
          (Default|DamageZone (Variables|State|GetZone) (Variables|Tuning|GetAttackDamage))
          (CallFunction|EnterState "NewEnumerator1")
          (else
            (CallFunction|EnterState "NewEnumerator1")))))))

(event EventBeginPlay
  (bind _stats (Variables|Default|GetStats))
  (Variables|Tuning|SetAttackDamage (Variables|/Game/Data/PDA_EnemyStats.PDA_EnemyStats_C|GetAttackDamage _stats))
  (Variables|Tuning|SetAttackCooldown (Variables|/Game/Data/PDA_EnemyStats.PDA_EnemyStats_C|GetAttackCooldown _stats))
  (Variables|Tuning|SetWindUpTime (Variables|/Game/Data/PDA_EnemyStats.PDA_EnemyStats_C|GetWindUpTime _stats))
  (|CallParentFunction)
  (bind _returnvalue (Actor|GetActorOfClass "/Game/BluePrints/BP_DefenceZone.BP_DefenceZone_C"))
  (Variables|State|SetZone _returnvalue)
  (CallFunction|TryClaimSlot))

(event Collision|EventActorBeginOverlap
  (params (OtherActor :type Actor%20Object%20Reference))
  (|CallParentFunction OtherActor) ; This node is disabled and will not be called.\nDrag off pins to build functionality.
)

(event EventTick
  (params (DeltaSeconds :type Float%20%28single-precision%29))
  (|CallParentFunction DeltaSeconds) ; This node is disabled and will not be called.\nDrag off pins to build functionality.
)

(event EventDie
  (CallFunction|EnterState "NewEnumerator4")
  (|CallParentFunction))

(fn ConstructionScript
  (|CallParentFunction))